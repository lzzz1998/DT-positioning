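; PC_Demo is a demo player controller that lets the user switch between the player character and a god-mode pawn.
; On BeginPlay it caches the current player pawn.
; Pressing Tab checks whether that pawn is a CH_Player, then possesses the stored god-mode pawn reference if so, or the stored player reference otherwise.
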(event `self.ReceiveBeginPlay`
  (set `self.ControlledPawn` (`GameplayStatics.GetPlayerPawn` 0)))

(event `Key|Tab`
  (params (Key :type "Key Structure"))
  (:`Pressed`
    (`self.Control Next Pawn`)))

(event `Control Next Pawn`
  ;[1 1 1] Switch Between GodMode Pawn and Player Pawn
  (cast `/Game/Characters/Player/CH_Player` (`self.ControlledPawn`)
    (:`then`
      (bind _output_get (set `self.ControlledPawn` (`self.CHGodModeRef`)))
      (`self.Possess` _output_get))
    (:`CastFailed`
      (bind _output_get_2 (set `self.ControlledPawn` (`self.CHPlayerRef`)))
      (`self.Possess` _output_get_2))))

(fn `UserConstructionScript`)